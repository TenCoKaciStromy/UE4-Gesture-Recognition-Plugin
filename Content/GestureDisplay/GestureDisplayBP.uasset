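; Gesture display actor that draws each gesture template as a 3D spline and shows live recognition progress on it.
; CreateSplines builds side-by-side spline components from each template's raw points, then adds spline meshes per segment, stored together in SplineCompStruct.
; Tick maps each template's EstimatedAlignment to a count of highlighted segments, turning the whole gesture green above a high threshold.
; SetColor and SetColorActivated repeat similar colouring on demand.
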(event EventTick
  (params (DeltaSeconds :type Float%20%28single-precision%29))
  (if (> (Utilities|Array|Length (Variables|Default|GetSplineCompStruct)) 0)
    (CallFunction|GetAllTemplates)
    (Variables|Default|SetGestureTemplates (Utilities|Array|MakeArray (Variables|Default|GetTemplateManager)))
    (for (_array_element _array_index) (Variables|Default|GetSplineCompStruct)
      (Variables|Default|SetMeshValue (Math|Float|Floor (* (- (Spline|GetNumberOfSplinePoints (.SplineComp (Utilities|Struct|BreakSplineStruct _array_element))) 1) (Variables|Default|GetestimatedAlignment (Utilities|Array|Get(acopy) 0 _array_index)))))
      (for (_array_element_2 _array_index_2) (.SplineMeshes (Utilities|Struct|BreakSplineStruct _array_element))
        (if (> (Variables|Default|GetestimatedAlignment (Utilities|Array|Get(acopy) 0 _array_index)) 0.94)
          (Rendering|Material|SetMaterial _array_element_2 0 "/Engine/EngineDebugMaterials/VertexColorViewMode_GreenOnly.VertexColorViewMode_GreenOnly")
          (elif (<= _array_index_2 (Variables|Default|GetMeshValue))
            (Rendering|Material|SetMaterial _array_element_2 0 (Variables|Default|GetHighlightMaterial))
            (else
              (Rendering|Material|SetMaterial _array_element_2 0 (Variables|Default|GetNormalMaterial)))))))))

(fn ConstructionScript)

(fn CreateSplines
  (params (GestureTemplates :type Array%20of%20%20Object%20References) (TemplateManager :type %20Object%20Reference))
  (bind _splinepointstemp (Variables|Default|GetSplinePointsTemp))
  (bind _splinecompstruct (Variables|Default|GetSplineCompStruct))
  (Variables|Default|SetTemplateManager 0)
  ;[1 1 1] Init
  (Variables|Default|SetGestureTemplates 0)
  (Variables|Default|SetSpawnTransform (Math|Transform|MakeTransform "0.000000, 0, 0"))
  (Utilities|Array|Clear (Variables|Default|GetSplineCompStruct))
  (Utilities|FlowControl|Sequence
    (:then_0
      ;[1 1 1] Create Spline comps for each gesture
      (for _array_element 0
        (bind _returnvalue (AddComponent|AddSplineComponent false (Variables|Default|GetSpawnTransform)))
        (Utilities|Array|Add (Variables|Default|GetSplineCompStruct) (Utilities|Struct|MakeSplineStruct (Utilities|Array|MakeArray 0) _returnvalue))
        ;[1 1 1] Resize points to bigger scale
        (Utilities|Array|Clear (Variables|Default|GetSplinePointsTemp))
        (for _array_element_2 (Variables|Default|GettemplateRaw _array_element)
          (Utilities|Array|Add _splinepointstemp (* _array_element_2 1.0)))
        (Spline|SetSplinePoints _returnvalue _splinepointstemp "Local" true)
        ;[1 1 1] Increment SPawn transform
        (Variables|Default|SetSpawnTransform (Math|Transform|MakeTransform (+ (.Location (Math|Transform|BreakTransform (Variables|Default|GetSpawnTransform))) (* (Math|Vector|GetRightVector (.Rotation (Math|Transform|BreakTransform (Variables|Default|GetSpawnTransform)))) 5e+01)) (.Rotation (Math|Transform|BreakTransform (Variables|Default|GetSpawnTransform))) (.Scale (Math|Transform|BreakTransform (Variables|Default|GetSpawnTransform)))))))
    (:then_1
      ;[1 1 1] Create Spline meshes for each comps
      (for (_array_element_3 _array_index) _splinecompstruct
        (Utilities|Array|Clear (Variables|Default|GetTemplSplineMeshComp))
        (for _index (range 0 (- (Spline|GetNumberOfSplinePoints (.SplineComp (Utilities|Struct|BreakSplineStruct _array_element_3))) 2))
          (bind _returnvalue_2 (AddComponent|AddSplineMeshComponent false (Transformation|GetRelativeTransform (.SplineComp (Utilities|Struct|BreakSplineStruct _array_element_3)))))
          (SplineMesh|SetStartandEnd _returnvalue_2 (.Location (Spline|GetLocationandTangentatSplinePoint (.SplineComp (Utilities|Struct|BreakSplineStruct _array_element_3)) _index "Local")) (.Tangent (Spline|GetLocationandTangentatSplinePoint (.SplineComp (Utilities|Struct|BreakSplineStruct _array_element_3)) _index "Local")) (.Location (Spline|GetLocationandTangentatSplinePoint (.SplineComp (Utilities|Struct|BreakSplineStruct _array_element_3)) (+ _index 1) "Local")) (.Tangent (Spline|GetLocationandTangentatSplinePoint (.SplineComp (Utilities|Struct|BreakSplineStruct _array_element_3)) (+ _index 1) "Local")) true :!class /Script/Engine.SplineMeshComponent)
          (Utilities|Array|Add (Variables|Default|GetTemplSplineMeshComp) _returnvalue_2))
        (Utilities|Array|SetArrayElem _splinecompstruct _array_index (Utilities|Struct|MakeSplineStruct (Variables|Default|GetTemplSplineMeshComp) (.SplineComp (Utilities|Struct|BreakSplineStruct _array_element_3))))))))

(fn Activated)

(fn SetColor
  (params (Condition :type Boolean))
  (if Condition
    (CallFunction|GetAllTemplates)
    (Variables|Default|SetGestureTemplates 0)
    (if (> (Utilities|Array|Length 0) 0)
      (for (_array_element _array_index) (Variables|Default|GetSplineCompStruct)
        (Variables|Default|SetMeshValue (Math|Float|Floor (* (- (Spline|GetNumberOfSplinePoints (.SplineComp (Utilities|Struct|BreakSplineStruct _array_element))) 1) (Variables|Default|GetestimatedAlignment (Utilities|Array|Get(acopy) 0 _array_index)))))
        (for (_array_element_2 _array_index_2) (.SplineMeshes (Utilities|Struct|BreakSplineStruct _array_element))
          (if (> (Variables|Default|GetestimatedAlignment (Utilities|Array|Get(acopy) 0 _array_index)) 0.9)
            (Rendering|Material|SetMaterial _array_element_2 0 "/Engine/EngineDebugMaterials/VertexColorViewMode_GreenOnly.VertexColorViewMode_GreenOnly")
            (elif (<= _array_index_2 (Variables|Default|GetMeshValue))
              (Rendering|Material|SetMaterial _array_element_2 0 (Variables|Default|GetHighlightMaterial))
              (else
                (Rendering|Material|SetMaterial _array_element_2 0 (Variables|Default|GetNormalMaterial))))))
        (return))))
  (return))

(fn SetColorActivated
  (params (Condition :type Boolean))
  (if Condition
    (CallFunction|GetAllTemplates)
    (Variables|Default|SetGestureTemplates 0)
    (if (> (Utilities|Array|Length 0) 0)
      (for (_array_element _array_index) (Variables|Default|GetSplineCompStruct)
        (Variables|Default|SetMeshValue (Math|Float|Floor (* (- (Spline|GetNumberOfSplinePoints (.SplineComp (Utilities|Struct|BreakSplineStruct _array_element))) 1) (Variables|Default|GetestimatedAlignment (Utilities|Array|Get(acopy) 0 _array_index)))))
        (for (_array_element_2 _array_index_2) (.SplineMeshes (Utilities|Struct|BreakSplineStruct _array_element))
          (if (<= _array_index_2 (Variables|Default|GetMeshValue))
            (Rendering|Material|SetMaterial _array_element_2 0 (Variables|Default|GetHighlightMaterial))
            (else
              (Rendering|Material|SetMaterial _array_element_2 0 (Variables|Default|GetNormalMaterial))))
          (return))
        (return))))
  (return))